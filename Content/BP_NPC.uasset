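; BP_NPC is a talkable NPC that registers itself with the player character and owns an AI chat component.
; Its TalkRange overlap sets the player's CurrentNPC and CanTalk on entry and clears them on exit.
; On BeginPlay it binds an AIChat reply event and sends a "Hello" message.
; The reply handler is empty, as the formatted chat-line output is left disconnected.
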(event OnComponentBeginOverlap(TalkRange)
  (params (OverlappedComponent :type Primitive%20Component%20Object%20Reference) (OtherActor :type Actor%20Object%20Reference) (OtherComp :type Primitive%20Component%20Object%20Reference) (OtherBodyIndex :type Integer) (bFromSweep :type Boolean) (SweepResult :type Hit%20Result%20Structure%20%28by%20ref%29))
  (bind _asbp_third_person_character (Utilities|Casting|CastToBP_ThirdPersonCharacter OtherActor))
  (Variables|/Game/ThirdPerson/Blueprints/BP_ThirdPersonCharacter.BP_ThirdPersonCharacter_C|SetCurrentNPC _asbp_third_person_character self)
  (Variables|/Game/ThirdPerson/Blueprints/BP_ThirdPersonCharacter.BP_ThirdPersonCharacter_C|SetCanTalk _asbp_third_person_character true))

(event OnComponentEndOverlap(TalkRange)
  (params (OverlappedComponent :type Primitive%20Component%20Object%20Reference) (OtherActor :type Actor%20Object%20Reference) (OtherComp :type Primitive%20Component%20Object%20Reference) (OtherBodyIndex :type Integer))
  (bind _asbp_third_person_character (Utilities|Casting|CastToBP_ThirdPersonCharacter OtherActor))
  (Variables|/Game/ThirdPerson/Blueprints/BP_ThirdPersonCharacter.BP_ThirdPersonCharacter_C|SetCanTalk _asbp_third_person_character false)
  (Variables|/Game/ThirdPerson/Blueprints/BP_ThirdPersonCharacter.BP_ThirdPersonCharacter_C|SetCurrentNPC _asbp_third_person_character 0))

(event Custom|自定义事件
  (params (Reply :type Text%20%28by%20ref%29)))

(event EventBeginPlay
  (bind _aichat (Variables|Default|GetAIChat))
  (EventDispatchers|BindEventtoOnReply _aichat (delegate Custom|自定义事件))
  (Class|AIChatComponent|SendChat _aichat (Utilities|Text|MakeLiteralText "Hello")))

(fn ConstructionScript)